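; Painter UV table actor with left and right doors that swing open and closed on interaction.
; ToggleDoor matches the hit component to a door, then plays or reverses that door's Timeline based on its open flag to drive relative yaw.
; The Timelines set the open flags to true, and nothing here clears them.
; A Box overlap adds an E interaction prompt for BP_ThirdPersonCharacter and removes all such prompts on exit.
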(event OnComponentBeginOverlap(Box)
  (params (OverlappedComponent :type Primitive%20Component%20Object%20Reference) (OtherActor :type Actor%20Object%20Reference) (OtherComp :type Primitive%20Component%20Object%20Reference) (OtherBodyIndex :type Integer) (bFromSweep :type Boolean) (SweepResult :type Hit%20Result%20Structure%20%28by%20ref%29))
  (Utilities|Casting|CastToBP_ThirdPersonCharacter OtherActor)
  (bind _returnvalue (UserInterface|CreateWidget "/Game/UI/Blueprints/WBP_InteractionPrompt_E.WBP_InteractionPrompt_E_C"))
  (UserInterface|Viewport|AddtoViewport _returnvalue 0))

(event OnComponentEndOverlap(Box)
  (params (OverlappedComponent :type Primitive%20Component%20Object%20Reference) (OtherActor :type Actor%20Object%20Reference) (OtherComp :type Primitive%20Component%20Object%20Reference) (OtherBodyIndex :type Integer))
  (Utilities|Casting|CastToBP_ThirdPersonCharacter OtherActor)
  (bind _foundwidgets (Widget|GetAllWidgetsOfClass "/Game/UI/Blueprints/WBP_InteractionPrompt_E.WBP_InteractionPrompt_E_C" true))
  (for _array_element _foundwidgets
    (Widget|RemovefromParent _array_element)))

(event Custom|ToggleDoor
  (params (HitComponent :type Primitive%20Component%20Object%20Reference))
  (if (== HitComponent (Variables|Default|GetRight%20Door))
    (if (Variables|Default|GetIsRightOpen)
      (bind _rightdoor (Timeline|Timeline Reverse)
        (:Update
          (Transformation|SetRelativeRotation (Variables|Default|GetRight%20Door) (Math|Rotator|MakeRotator 0.0 0.0 (+ _rightdoor -1.8e+02)) false false))
        (:Finished
          _))
      (Variables|Default|SetIsRightOpen true)
      (else
        (Timeline|Timeline Play)))
    (elif (== HitComponent (Variables|Default|GetLeft%20Door))
      (if (Variables|Default|GetIsLeftOpen)
        (bind _leftdoor (Timeline|Timeline_0 Reverse)
          (:Update
            (Transformation|SetRelativeRotation (Variables|Default|GetLeft%20Door) (Math|Rotator|MakeRotator 0.0 0.0 _leftdoor) false false))
          (:Finished
            _))
        (Variables|Default|SetIsLeftOpen true)
        (else
          (Timeline|Timeline_0 Play))))))

(event EventBeginPlay)

(event Collision|EventActorBeginOverlap
  (params (OtherActor :type Actor%20Object%20Reference)))

(event EventTick
  (params (DeltaSeconds :type Float%20%28single-precision%29)))

(fn ConstructionScript)