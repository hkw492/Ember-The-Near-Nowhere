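; BP_MemoryObject is an interactable world object that shows a memory image when the player presses E nearby.
; Its TriggerZone shows an interaction prompt and enables input when the third-person character enters.
; E swaps the prompt for a popup displaying MemoryTexture, switches to UI-only input with cursor, and applies a glow overlay to the mesh.
; Leaving removes prompts and, if a popup is valid, closes it, restores game input and disables the actor's input.
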(event OnComponentBeginOverlap(TriggerZone)
  (params (OverlappedComponent :type Primitive%20Component%20Object%20Reference) (OtherActor :type Actor%20Object%20Reference) (OtherComp :type Primitive%20Component%20Object%20Reference) (OtherBodyIndex :type Integer) (bFromSweep :type Boolean) (SweepResult :type Hit%20Result%20Structure%20%28by%20ref%29))
  (Utilities|Casting|CastToBP_ThirdPersonCharacter OtherActor)
  (bind _returnvalue (UserInterface|CreateWidget "/Game/UI/Blueprints/WBP_InteractionPrompt_E.WBP_InteractionPrompt_E_C"))
  (bind _output_get (Variables|Default|SetPromptWidget _returnvalue))
  (UserInterface|Viewport|AddtoViewport _output_get 0)
  (Input|EnableInput (Game|GetPlayerController 0)))

(event OnComponentEndOverlap(TriggerZone)
  (params (OverlappedComponent :type Primitive%20Component%20Object%20Reference) (OtherActor :type Actor%20Object%20Reference) (OtherComp :type Primitive%20Component%20Object%20Reference) (OtherBodyIndex :type Integer))
  (bind _returnvalue (Game|GetPlayerController 0))
  (bind _popupwidget (Variables|Default|GetPopupWidget))
  (Utilities|Casting|CastToBP_ThirdPersonCharacter OtherActor)
  (bind _foundwidgets (Widget|GetAllWidgetsOfClass "/Game/UI/Blueprints/WBP_InteractionPrompt_E.WBP_InteractionPrompt_E_C" true))
  (for _array_element _foundwidgets
    (Widget|RemovefromParent _array_element))
  (Utilities|IsValid _popupwidget
    (:Is%20Valid
      (Widget|RemovefromParent _popupwidget)
      (Input|SetInputModeGameOnly _returnvalue false)
      (Variables|/Script/Engine.PlayerController|SetbShowMouseCursor _returnvalue false)
      (Variables|Default|SetIsViewing false)
      (Input|DisableInput _returnvalue))))

(event EventBeginPlay)

(event Collision|EventActorBeginOverlap
  (params (OtherActor :type Actor%20Object%20Reference)))

(event EventTick
  (params (DeltaSeconds :type Float%20%28single-precision%29)))

(event Input|KeyboardEvents|E
  (params (Key :type Key%20Structure :default "None"))
  (bind _returnvalue (Game|GetPlayerController 0))
  (:Pressed
    (if (not (Variables|Default|GetIsViewing))
      (bind _foundwidgets (Widget|GetAllWidgetsOfClass "/Game/UI/Blueprints/WBP_InteractionPrompt_E.WBP_InteractionPrompt_E_C" true))
      (for _array_element _foundwidgets
        (Widget|RemovefromParent _array_element))
      (bind _returnvalue_2 (UserInterface|CreateWidget "/Game/UI/Blueprints/WBP_MemoryPopup.WBP_MemoryPopup_C" 0 (Variables|Default|GetMemoryTexture)))
      (bind _output_get (Variables|Default|SetPopupWidget _returnvalue_2))
      (UserInterface|Viewport|AddtoViewport _output_get 0)
      (Input|SetInputModeUIOnly _returnvalue _output_get "DoNotLock" false)
      (Variables|/Script/Engine.PlayerController|SetbShowMouseCursor _returnvalue true)
      (Variables|Default|SetIsViewing true)
      (Rendering|Material|SetOverlayMaterial (Variables|Default|GetStaticMesh) "/Game/Textures/Glow_Box/M_Interactable_Glow.M_Interactable_Glow" :!class /Script/Engine.MeshComponent))))

(fn ConstructionScript)