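; Inventory component that stores items in a two-slot map keyed by slot index.
; AddItem fills the first free slot and broadcasts OnInventoryUpdated, or shows an "Inventory is full" flash widget and reports failure.
; RemoveItem clears a slot without broadcasting, and HasItem uses FindSlotOfItem to search by ItemID, treating a positive slot as found.
; PlaceItem is an empty stub.
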(event EventBeginPlay)

(event EventTick
  (params (DeltaSeconds :type Float%20%28single-precision%29)))

(fn AddItem
  (params (ItemToAdd :type S%20Item%20Details%20Structure))
  (bind _inventorymap (Variables|Default|GetInventoryMap))
  (for _index (range 1 2)
    (if (not (Utilities|Map|Contains _inventorymap _index))
      (Utilities|Map|Add _inventorymap _index ItemToAdd)
      (Default|CallOnInventoryUpdated _index ItemToAdd)
      (return true _index)))
  (bind _returnvalue (UserInterface|CreateWidget "/Game/UI/Blueprints/WBP_FlashMessage.WBP_FlashMessage_C" 0 "Inventory is full"))
  (UserInterface|Viewport|AddtoViewport _returnvalue 0)
  (return false -1))

(fn PlaceItem
  (params (ItemToPlace :type S%20Item%20Details%20Structure)))

(fn RemoveItem
  (params (SlotToRemove :type Integer))
  (Utilities|Map|Remove (Variables|Default|GetInventoryMap) SlotToRemove)
  (return))

(fn HasItem
  (params (TargetItemID :type Integer))
  (bind _slotindex (CallFunction|FindSlotOfItem TargetItemID))
  (return (> _slotindex 0)))

(fn FindSlotOfItem
  (params (TargetItemID :type Integer))
  (bind _inventorymap (Variables|Default|GetInventoryMap))
  (bind _keys (Utilities|Map|Keys _inventorymap))
  (for _array_element _keys
    (if (== (.ItemID (Utilities|Struct|BreakS_ItemDetails (.Value (Utilities|Map|Find _inventorymap _array_element)))) TargetItemID)
      (return _array_element))))