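; BP_BirdHouse is an interactable bird house actor that is always available for interaction.
; Its interaction events toggle an overlay on the static mesh: OnInteractEnd applies the green highlight material, while OnInteractHighlight clears it, the reverse of what the event names suggest.
; CanInteract always returns true, and the construction script only calls its parent.
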(event EventBeginPlay
  (|CallParentFunction) ; This node is disabled and will not be called.\nDrag off pins to build functionality.
)

(event Collision|EventActorBeginOverlap
  (params (OtherActor :type Actor%20Object%20Reference))
  (|CallParentFunction OtherActor) ; This node is disabled and will not be called.\nDrag off pins to build functionality.
)

(event EventTick
  (params (DeltaSeconds :type Float%20%28single-precision%29))
  (|CallParentFunction DeltaSeconds) ; This node is disabled and will not be called.\nDrag off pins to build functionality.
)

(event EventOnInteractEnd
  (Rendering|Material|SetOverlayMaterial (Variables|Default|GetStaticMesh) "/Game/Textures/Glow_Box/MI_GreenHighlight.MI_GreenHighlight" :!class /Script/Engine.MeshComponent))

(event EventOnInteractHighlight
  (Rendering|Material|SetOverlayMaterial (Variables|Default|GetStaticMesh) 0 :!class /Script/Engine.MeshComponent))

(fn ConstructionScript
  (|CallParentFunction))

(fn CanInteract
  (return true))