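; BP_Upper_NPC is an NPC actor that highlights on approach and opens the WBP_Father widget from a trigger.
; Its CHAWITHBONE mesh starts with a faint glow material and switches to full glow when anything overlaps Sphere.
; Leaving Sphere applies the Cha_With_Bon material and destroys the sphere, ending the highlight.
; The Cutscene trigger adds the widget to the viewport when BP_ThirdPersonCharacter enters, then destroys itself to fire once.
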(event OnComponentBeginOverlap(Sphere)
  (params (OverlappedComponent :type Primitive%20Component%20Object%20Reference) (OtherActor :type Actor%20Object%20Reference) (OtherComp :type Primitive%20Component%20Object%20Reference) (OtherBodyIndex :type Integer) (bFromSweep :type Boolean) (SweepResult :type Hit%20Result%20Structure%20%28by%20ref%29))
  (Rendering|Material|SetMaterial (Variables|Default|GetCHA_WITH_BONE) 0 "/Game/Textures/Glow_Box/M_Interactable_Glow.M_Interactable_Glow"))

(event OnComponentEndOverlap(Sphere)
  (params (OverlappedComponent :type Primitive%20Component%20Object%20Reference) (OtherActor :type Actor%20Object%20Reference) (OtherComp :type Primitive%20Component%20Object%20Reference) (OtherBodyIndex :type Integer))
  (Rendering|Material|SetMaterial (Variables|Default|GetCHA_WITH_BONE) 0 "/Game/Characters/Cha_With_Bon.Cha_With_Bon")
  (Components|DestroyComponent (Variables|Default|GetSphere)))

(event OnComponentBeginOverlap(Cutscene)
  (params (OverlappedComponent :type Primitive%20Component%20Object%20Reference) (OtherActor :type Actor%20Object%20Reference) (OtherComp :type Primitive%20Component%20Object%20Reference) (OtherBodyIndex :type Integer) (bFromSweep :type Boolean) (SweepResult :type Hit%20Result%20Structure%20%28by%20ref%29))
  (Utilities|Casting|CastToBP_ThirdPersonCharacter OtherActor)
  (bind _returnvalue (UserInterface|CreateWidget "/Game/UI/Blueprints/WBP_Father.WBP_Father_C"))
  (UserInterface|Viewport|AddtoViewport _returnvalue 0)
  (Components|DestroyComponent (Variables|Default|GetCutscene)))

(event EventBeginPlay
  (Rendering|Material|SetMaterial (Variables|Default|GetCHA_WITH_BONE) 0 "/Game/Textures/Glow_Box/M_Interactable_Glow_Min.M_Interactable_Glow_Min"))

(event Collision|EventActorBeginOverlap
  (params (OtherActor :type Actor%20Object%20Reference)))

(event EventTick
  (params (DeltaSeconds :type Float%20%28single-precision%29)))

(fn ConstructionScript)