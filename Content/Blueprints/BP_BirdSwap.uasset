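; Clickable bird-swap puzzle actor where three crows and three ravens must trade sides across seven pins.
; Crows move only right and ravens only left, sliding one pin or jumping two into the gap, tracked in parallel state and mesh arrays.
; Trigger overlap shows an interaction prompt, and enter/exit events manage a temporary camera, cursor and exit widget.
; Solving reveals TargetFrame, exits the view, and updates the character's solved flag and objective.
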(event OnClicked(Crow_L1)
  (params (TouchedComponent :type Primitive%20Component%20Object%20Reference) (ButtonPressed :type Key%20Structure :default "None"))
  (CallFunction|TryMoveBird (Utilities|Array|FindItem (Variables|Default|GetBirdLocations) (Variables|Default|GetCrow_L1))))

(event OnClicked(Crow_L2)
  (params (TouchedComponent :type Primitive%20Component%20Object%20Reference) (ButtonPressed :type Key%20Structure :default "None"))
  (CallFunction|TryMoveBird (Utilities|Array|FindItem (Variables|Default|GetBirdLocations) (Variables|Default|GetCrow_L2))))

(event OnClicked(Crow_L3)
  (params (TouchedComponent :type Primitive%20Component%20Object%20Reference) (ButtonPressed :type Key%20Structure :default "None"))
  (CallFunction|TryMoveBird (Utilities|Array|FindItem (Variables|Default|GetBirdLocations) (Variables|Default|GetCrow_L3))))

(event OnClicked(Raven_R1)
  (params (TouchedComponent :type Primitive%20Component%20Object%20Reference) (ButtonPressed :type Key%20Structure :default "None"))
  (CallFunction|TryMoveBird (Utilities|Array|FindItem (Variables|Default|GetBirdLocations) (Variables|Default|GetRaven_R1))))

(event OnClicked(Raven_R2)
  (params (TouchedComponent :type Primitive%20Component%20Object%20Reference) (ButtonPressed :type Key%20Structure :default "None"))
  (CallFunction|TryMoveBird (Utilities|Array|FindItem (Variables|Default|GetBirdLocations) (Variables|Default|GetRaven_R2))))

(event OnClicked(Raven_R3)
  (params (TouchedComponent :type Primitive%20Component%20Object%20Reference) (ButtonPressed :type Key%20Structure :default "None"))
  (CallFunction|TryMoveBird (Utilities|Array|FindItem (Variables|Default|GetBirdLocations) (Variables|Default|GetRaven_R3))))

(event OnComponentBeginOverlap(Trigger)
  (params (OverlappedComponent :type Primitive%20Component%20Object%20Reference) (OtherActor :type Actor%20Object%20Reference) (OtherComp :type Primitive%20Component%20Object%20Reference) (OtherBodyIndex :type Integer) (bFromSweep :type Boolean) (SweepResult :type Hit%20Result%20Structure%20%28by%20ref%29))
  (Utilities|Casting|CastToBP_ThirdPersonCharacter OtherActor)
  (bind _returnvalue (UserInterface|CreateWidget "/Game/UI/Blueprints/WBP_InteractionPrompt_E.WBP_InteractionPrompt_E_C"))
  (bind _output_get (Variables|Default|SetInteractionWidgetRef _returnvalue))
  (UserInterface|Viewport|AddtoViewport _output_get 0))

(event OnComponentEndOverlap(Trigger)
  (params (OverlappedComponent :type Primitive%20Component%20Object%20Reference) (OtherActor :type Actor%20Object%20Reference) (OtherComp :type Primitive%20Component%20Object%20Reference) (OtherBodyIndex :type Integer))
  (Utilities|Casting|CastToBP_ThirdPersonCharacter OtherActor)
  (bind _foundwidgets (Widget|GetAllWidgetsOfClass "/Game/UI/Blueprints/WBP_InteractionPrompt_E.WBP_InteractionPrompt_E_C" true))
  (for _array_element _foundwidgets
    (Widget|RemovefromParent _array_element)))

(event Custom|TryMoveBird
  (params (CurrentIndex :type Integer))
  (switch int (Utilities|Array|Get(acopy) (Variables|Default|GetGridState) CurrentIndex)
    (:1
      (Variables|Default|SetDir 1))
    (:2
      (Variables|Default|SetDir -1)))
  (Variables|Default|SetTargetSlide (+ CurrentIndex (Variables|Default|GetDir)))
  (if (Math|Integer|InRange(Integer) (Variables|Default|GetTargetSlide) 0 6)
    (if (== (Utilities|Array|Get(acopy) (Variables|Default|GetGridState) (Variables|Default|GetTargetSlide)) 0)
      (CallFunction|PerformSwap CurrentIndex (Variables|Default|GetTargetSlide))
      (else
        (bind _output_get (Variables|Default|SetTargetJump (+ CurrentIndex (* (Variables|Default|GetDir) 2)) :!label _label))
        (if (Math|Integer|InRange(Integer) _output_get 0 6)
          (if (== (Utilities|Array|Get(acopy) (Variables|Default|GetGridState) (Variables|Default|GetTargetJump)) 0)
            (CallFunction|PerformSwap CurrentIndex (Variables|Default|GetTargetJump))))))
    (else
      (goto _label))))

(event Custom|CheckWinCondition
  (bind _targetframe (Variables|Default|GetTargetFrame))
  (bind _gridstate (Variables|Default|GetGridState))
  (if (Math|Boolean|ANDBoolean (== (Utilities|Array|Get(acopy) _gridstate) 2) (== (Utilities|Array|Get(acopy) _gridstate 1) 2) (== (Utilities|Array|Get(acopy) _gridstate 2) 2) (== (Utilities|Array|Get(acopy) _gridstate 4) 1) (== (Utilities|Array|Get(acopy) _gridstate 5) 1) (== (Utilities|Array|Get(acopy) _gridstate 6) 1))
    (Rendering|SetActorHiddenInGame _targetframe false)
    (Game|Player|SetViewTargetwithBlend (Game|GetPlayerController 0) _targetframe 1.0 "VTBlend_Linear" 0.0 false)
    (Utilities|FlowControl|Delay 3.0)
    (CallFunction|ExitPuzzleView)
    (bind _asbp_third_person_character (Utilities|Casting|CastToBP_ThirdPersonCharacter (Game|GetPlayerCharacter 0)))
    (Variables|/Game/ThirdPerson/Blueprints/BP_ThirdPersonCharacter.BP_ThirdPersonCharacter_C|SetIsBirdSolved _asbp_third_person_character true)
    (Default|UpdateObjective _asbp_third_person_character "Use the clue to find the grave.")))

(event Custom|EnterPuzzleView
  (bind _returnvalue (Game|GetPlayerController 0))
  (bind _returnvalue_2 (Game|SpawnActorfromClass "/Script/Engine.CameraActor" (Transformation|GetWorldTransform (Variables|Default|GetPuzzleCamera)) "AlwaysSpawn" "MultiplyWithRoot" 0 0))
  (bind _output_get (Variables|Default|SetTempCameraActor _returnvalue_2))
  (Game|Player|SetViewTargetwithBlend _returnvalue _output_get 1.0 "VTBlend_Linear" 0.0 false)
  (Variables|/Script/Engine.PlayerController|SetbShowMouseCursor _returnvalue true)
  (Input|SetInputModeGameandUI _returnvalue 0 "DoNotLock" true false)
  (bind _returnvalue_3 (UserInterface|CreateWidget "/Game/UI/Blueprints/WBP_PuzzleExit_GY.WBP_PuzzleExit_GY_C"))
  (bind _output_get_2 (Variables|Default|SetExitWidgetRef _returnvalue_3))
  (UserInterface|Viewport|AddtoViewport _output_get_2 0)
  (bind _foundwidgets (Widget|GetAllWidgetsOfClass "/Game/UI/Blueprints/WBP_InteractionPrompt_E.WBP_InteractionPrompt_E_C" true))
  (for _array_element _foundwidgets
    (Widget|RemovefromParent _array_element)))

(event Custom|ExitPuzzleView
  (bind _returnvalue (Game|GetPlayerController 0))
  (Game|Player|SetViewTargetwithBlend _returnvalue (Game|GetPlayerCharacter 0) 1.0 "VTBlend_Linear" 0.0 false)
  (Actor|DestroyActor (Variables|Default|GetTempCameraActor))
  (Variables|/Script/Engine.PlayerController|SetbShowMouseCursor _returnvalue false)
  (Widget|RemovefromParent (Variables|Default|GetExitWidgetRef))
  (Input|SetInputModeGameOnly _returnvalue false))

(event Custom|ResetPuzzle
  (Components|MoveComponentTo (Variables|Default|GetCrow_L1) (Variables|/Script/Engine.SceneComponent|GetRelativeLocation (Variables|Default|GetPin_0)) "0, 0, 0" false false 0.5 false)
  (Components|MoveComponentTo (Variables|Default|GetCrow_L2) (Variables|/Script/Engine.SceneComponent|GetRelativeLocation (Variables|Default|GetPin_1)) "0, 0, 0" false false 0.5 false)
  (Components|MoveComponentTo (Variables|Default|GetCrow_L3) (Variables|/Script/Engine.SceneComponent|GetRelativeLocation (Variables|Default|GetPin_2)) "0, 0, 0" false false 0.5 false)
  (Components|MoveComponentTo (Variables|Default|GetRaven_R1) (Variables|/Script/Engine.SceneComponent|GetRelativeLocation (Variables|Default|GetPin_4)) "0, 0, 0" false false 0.5 false)
  (Components|MoveComponentTo (Variables|Default|GetRaven_R2) (Variables|/Script/Engine.SceneComponent|GetRelativeLocation (Variables|Default|GetPin_5)) "0, 0, 0" false false 0.5 false)
  (Components|MoveComponentTo (Variables|Default|GetRaven_R3) (Variables|/Script/Engine.SceneComponent|GetRelativeLocation (Variables|Default|GetPin_6)) "0, 0, 0" false false 0.5 false)
  (Variables|Default|SetGridState (Utilities|Array|MakeArray 1 1 1 0 2 2 2))
  (Variables|Default|SetBirdLocations (Utilities|Array|MakeArray (Variables|Default|GetCrow_L1) (Variables|Default|GetCrow_L2) (Variables|Default|GetCrow_L3) 0 (Variables|Default|GetRaven_R1) (Variables|Default|GetRaven_R2) (Variables|Default|GetRaven_R3))))

(event Custom|PerformSwap
  (params (FromIndex :type Integer) (ToIndex :type Integer))
  (bind _birdlocations (Variables|Default|GetBirdLocations))
  (bind _gridstate (Variables|Default|GetGridState))
  (Variables|Default|SetMovingMesh (Utilities|Array|Get(acopy) _birdlocations FromIndex))
  (Utilities|Array|SetArrayElem _gridstate ToIndex (Utilities|Array|Get(acopy) _gridstate FromIndex))
  (Utilities|Array|SetArrayElem _gridstate FromIndex 0)
  (Utilities|Array|SetArrayElem _birdlocations ToIndex (Variables|Default|GetMovingMesh))
  (Utilities|Array|SetArrayElem _birdlocations FromIndex 0)
  (Components|MoveComponentTo (Variables|Default|GetMovingMesh) (Variables|/Script/Engine.SceneComponent|GetRelativeLocation (Utilities|Select :Index ToIndex :Option%200 (Variables|Default|GetPin_0) :Option%201 (Variables|Default|GetPin_1) :Option%202 (Variables|Default|GetPin_2) :Option%203 (Variables|Default|GetPin_3) :Option%204 (Variables|Default|GetPin_4) :Option%205 (Variables|Default|GetPin_5) :Option%206 (Variables|Default|GetPin_6))) "0, 0, 0" true false 0.3 false)
  (CallFunction|CheckWinCondition))

(event EventBeginPlay
  (Variables|Default|SetBirdLocations (Utilities|Array|MakeArray (Variables|Default|GetCrow_L1) (Variables|Default|GetCrow_L2) (Variables|Default|GetCrow_L3) 0 (Variables|Default|GetRaven_R1) (Variables|Default|GetRaven_R2) (Variables|Default|GetRaven_R3)))
  (Variables|Default|SetGridState (Utilities|Array|MakeArray 1 1 1 0 2 2 2)))

(event Collision|EventActorBeginOverlap
  (params (OtherActor :type Actor%20Object%20Reference)))

(event EventTick
  (params (DeltaSeconds :type Float%20%28single-precision%29)))

(fn ConstructionScript)