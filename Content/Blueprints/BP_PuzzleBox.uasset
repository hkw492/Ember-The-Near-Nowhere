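; Puzzle box actor that shows an interact prompt on overlap and holds a four-button code puzzle rewarding the tombstone scroll.
; EnterPuzzleView blends to a temporary camera with cursor and exit widget, and clickable components feed PressButton, which compares the entered sequence with CorrectSequence.
; A wrong code flashes a message and resets input.
; Success swings the lid open by timeline, briefly shows the letter, adds the scroll to inventory and sets the graveyard objective.
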(event OnClicked(Btn1)
  (params (TouchedComponent :type Primitive%20Component%20Object%20Reference) (ButtonPressed :type Key%20Structure :default "None"))
  (CallFunction|PressButton 1))

(event OnClicked(Btn2)
  (params (TouchedComponent :type Primitive%20Component%20Object%20Reference) (ButtonPressed :type Key%20Structure :default "None"))
  (CallFunction|PressButton 2))

(event OnClicked(Btn3)
  (params (TouchedComponent :type Primitive%20Component%20Object%20Reference) (ButtonPressed :type Key%20Structure :default "None"))
  (CallFunction|PressButton 3))

(event OnClicked(Btn4)
  (params (TouchedComponent :type Primitive%20Component%20Object%20Reference) (ButtonPressed :type Key%20Structure :default "None"))
  (CallFunction|PressButton 4))

(event OnClicked(Img1)
  (params (TouchedComponent :type Primitive%20Component%20Object%20Reference) (ButtonPressed :type Key%20Structure :default "None"))
  (CallFunction|PressButton 1))

(event OnClicked(Img2)
  (params (TouchedComponent :type Primitive%20Component%20Object%20Reference) (ButtonPressed :type Key%20Structure :default "None"))
  (CallFunction|PressButton 2))

(event OnClicked(Img3)
  (params (TouchedComponent :type Primitive%20Component%20Object%20Reference) (ButtonPressed :type Key%20Structure :default "None"))
  (CallFunction|PressButton 3))

(event OnClicked(Img4)
  (params (TouchedComponent :type Primitive%20Component%20Object%20Reference) (ButtonPressed :type Key%20Structure :default "None"))
  (CallFunction|PressButton 4))

(event OnComponentBeginOverlap(InteractTrigger)
  (params (OverlappedComponent :type Primitive%20Component%20Object%20Reference) (OtherActor :type Actor%20Object%20Reference) (OtherComp :type Primitive%20Component%20Object%20Reference) (OtherBodyIndex :type Integer) (bFromSweep :type Boolean) (SweepResult :type Hit%20Result%20Structure%20%28by%20ref%29))
  (Utilities|Casting|CastToBP_ThirdPersonCharacter OtherActor)
  (bind _returnvalue (UserInterface|CreateWidget "/Game/UI/Blueprints/WBP_InteractionPrompt_E.WBP_InteractionPrompt_E_C"))
  (bind _output_get (Variables|Default|SetInteractWidRef _returnvalue))
  (UserInterface|Viewport|AddtoViewport _output_get 0))

(event OnComponentEndOverlap(InteractTrigger)
  (params (OverlappedComponent :type Primitive%20Component%20Object%20Reference) (OtherActor :type Actor%20Object%20Reference) (OtherComp :type Primitive%20Component%20Object%20Reference) (OtherBodyIndex :type Integer))
  (Utilities|Casting|CastToBP_ThirdPersonCharacter OtherActor)
  (bind _foundwidgets (Widget|GetAllWidgetsOfClass "/Game/UI/Blueprints/WBP_InteractionPrompt_E.WBP_InteractionPrompt_E_C" true))
  (for _array_element _foundwidgets
    (Widget|RemovefromParent _array_element)))

(event Custom|PressButton
  (params (ButtonID :type Integer))
  (bind _playersequence (Variables|Default|GetPlayerSequence))
  (if (not (Variables|Default|GetIsSolved))
    (Utilities|Array|Add _playersequence ButtonID)
    (Audio|PlaySound2D "/Game/Audio/Sounds/Single_Click.Single_Click" 1.0 1.0 0.0 0 0)
    (if (== (Utilities|Array|Length _playersequence) 4)
      (if (Math|Boolean|ANDBoolean (== (Utilities|Array|Get(acopy) (Variables|Default|GetPlayerSequence)) (Utilities|Array|Get(acopy) (Variables|Default|GetCorrectSequence))) (== (Utilities|Array|Get(acopy) (Variables|Default|GetPlayerSequence) 1) (Utilities|Array|Get(acopy) (Variables|Default|GetCorrectSequence) 1)) (== (Utilities|Array|Get(acopy) (Variables|Default|GetPlayerSequence) 2) (Utilities|Array|Get(acopy) (Variables|Default|GetCorrectSequence) 2)) (== (Utilities|Array|Get(acopy) (Variables|Default|GetPlayerSequence) 3) (Utilities|Array|Get(acopy) (Variables|Default|GetCorrectSequence) 3)))
        (Components|DestroyComponent (Variables|Default|GetInteract%20Trigger))
        (Variables|Default|SetIsSolved true)
        (bind _rotationalpha (Timeline|Open%20Lid Play)
          (:Update
            (Transformation|SetRelativeRotation (Variables|Default|GetLidHinge) (Math|Rotator|MakeRotator 0.0 (Math|Float|Lerp 0.0 1.1e+02 _rotationalpha) 0.0) false false))
          (:Finished
            (Development|SetHiddeninGame (Variables|Default|GetScrollMesh) false false)
            (bind _returnvalue (UserInterface|CreateWidget "/Game/UI/Blueprints/WBP_ScrollLetter.WBP_ScrollLetter_C"))
            (UserInterface|Viewport|AddtoViewport _returnvalue 0)
            (Variables|/Script/Engine.PlayerController|SetbShowMouseCursor (Game|GetPlayerController 0) true)
            (Utilities|FlowControl|Delay 3.0)
            (Development|SetHiddeninGame (Variables|Default|GetScrollMesh) true false)
            (bind _asbp_third_person_character (Utilities|Casting|CastToBP_ThirdPersonCharacter (Game|GetPlayerCharacter 0)))
            (Default|DiscardFlashlight _asbp_third_person_character)
            (Default|AddItem (Variables|/Game/ThirdPerson/Blueprints/BP_ThirdPersonCharacter.BP_ThirdPersonCharacter_C|GetBPC_Inventory _asbp_third_person_character) (Utilities|Struct|MakeS_ItemDetails 69 "Scroll" "/Game/Textures/Level_2/Graveyard/Tomb/Scroll_icon.Scroll_icon" "/Game/Textures/Level_2/Painting_and_Box_Puzzle/Scroll_.Scroll_"))
            (Variables|/Game/ThirdPerson/Blueprints/BP_ThirdPersonCharacter.BP_ThirdPersonCharacter_C|SetHasTombstoneScroll _asbp_third_person_character true)
            (Widget|RemovefromParent _returnvalue)
            (CallFunction|ExitPuzzleView)
            (Default|UpdateObjective _asbp_third_person_character "Go to the Graveyard")))
        (else
          (bind _returnvalue_2 (UserInterface|CreateWidget "/Game/UI/Blueprints/WBP_FlashMessage.WBP_FlashMessage_C" 0 "Wrong Code"))
          (UserInterface|Viewport|AddtoViewport _returnvalue_2 0)
          (Utilities|Array|Clear (Variables|Default|GetPlayerSequence)))))))

(event Custom|EnterPuzzleView
  (bind _returnvalue (Game|GetPlayerController 0))
  (bind _returnvalue_2 (Game|SpawnActorfromClass "/Script/Engine.CameraActor" (Transformation|GetWorldTransform (Variables|Default|GetPuzzleCamera)) "AlwaysSpawn" "MultiplyWithRoot" 0 0))
  (bind _output_get (Variables|Default|SetTempCameraActor _returnvalue_2))
  (Game|Player|SetViewTargetwithBlend _returnvalue _output_get 1.0 "VTBlend_Linear" 0.0 false)
  (Variables|/Script/Engine.PlayerController|SetbShowMouseCursor _returnvalue true)
  (Input|SetInputModeGameandUI _returnvalue 0 "DoNotLock" true false)
  (bind _returnvalue_3 (UserInterface|CreateWidget "/Game/UI/Blueprints/WBP_PuzzleExit.WBP_PuzzleExit_C"))
  (bind _output_get_2 (Variables|Default|SetExitWidgetRef _returnvalue_3))
  (UserInterface|Viewport|AddtoViewport _output_get_2 0))

(event Custom|ExitPuzzleView
  (bind _returnvalue (Game|GetPlayerController 0))
  (Game|Player|SetViewTargetwithBlend _returnvalue (Game|GetPlayerCharacter 0) 1.0 "VTBlend_Linear" 0.0 false)
  (Actor|DestroyActor (Variables|Default|GetTempCameraActor))
  (Variables|/Script/Engine.PlayerController|SetbShowMouseCursor _returnvalue false)
  (Input|SetInputModeGameOnly _returnvalue false)
  (Widget|RemovefromParent (Variables|Default|GetExitWidgetRef)))

(event EventBeginPlay)

(event Collision|EventActorBeginOverlap
  (params (OtherActor :type Actor%20Object%20Reference)))

(event EventTick
  (params (DeltaSeconds :type Float%20%28single-precision%29)))

(fn ConstructionScript)