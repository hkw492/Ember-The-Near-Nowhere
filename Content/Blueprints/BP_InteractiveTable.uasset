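; Interactive table actor with two openable drawers and a crafting zone for assembling a hammer.
; Overlap volumes enable input, select the current drawer and show or remove the table widget.
; F slides the selected drawer open through a timeline lerp from its cached start position.
; C spawns the whole hammer once both child-actor placement spots are filled, removing those spots, otherwise flashes a missing-parts message.
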(event OnComponentBeginOverlap(Trigger_Drawer1)
  (params (OverlappedComponent :type Primitive%20Component%20Object%20Reference) (OtherActor :type Actor%20Object%20Reference) (OtherComp :type Primitive%20Component%20Object%20Reference) (OtherBodyIndex :type Integer) (bFromSweep :type Boolean) (SweepResult :type Hit%20Result%20Structure%20%28by%20ref%29))
  (Variables|Default|SetCurrentDrawerIndex 1)
  (Input|EnableInput (Game|GetPlayerController 0)))

(event OnComponentBeginOverlap(Trigger_Drawer2)
  (params (OverlappedComponent :type Primitive%20Component%20Object%20Reference) (OtherActor :type Actor%20Object%20Reference) (OtherComp :type Primitive%20Component%20Object%20Reference) (OtherBodyIndex :type Integer) (bFromSweep :type Boolean) (SweepResult :type Hit%20Result%20Structure%20%28by%20ref%29))
  (Variables|Default|SetCurrentDrawerIndex 2)
  (Input|EnableInput (Game|GetPlayerController 0)))

(event OnComponentBeginOverlap(Input)
  (params (OverlappedComponent :type Primitive%20Component%20Object%20Reference) (OtherActor :type Actor%20Object%20Reference) (OtherComp :type Primitive%20Component%20Object%20Reference) (OtherBodyIndex :type Integer) (bFromSweep :type Boolean) (SweepResult :type Hit%20Result%20Structure%20%28by%20ref%29))
  (Utilities|Casting|CastToBP_ThirdPersonCharacter OtherActor)
  (bind _returnvalue (UserInterface|CreateWidget "/Game/UI/Blueprints/WBP_Interactive_Table.WBP_Interactive_Table_C"))
  (UserInterface|Viewport|AddtoViewport _returnvalue 0)
  (Input|EnableInput (Game|GetPlayerController 0)))

(event OnComponentEndOverlap(Input)
  (params (OverlappedComponent :type Primitive%20Component%20Object%20Reference) (OtherActor :type Actor%20Object%20Reference) (OtherComp :type Primitive%20Component%20Object%20Reference) (OtherBodyIndex :type Integer))
  (Utilities|Casting|CastToBP_ThirdPersonCharacter OtherActor)
  (bind _foundwidgets (Widget|GetAllWidgetsOfClass "/Game/UI/Blueprints/WBP_Interactive_Table.WBP_Interactive_Table_C" true))
  (for _array_element _foundwidgets
    (Widget|RemovefromParent _array_element))
  (Input|DisableInput (Game|GetPlayerController 0)))

(event OnComponentEndOverlap(Trigger_Drawer1)
  (params (OverlappedComponent :type Primitive%20Component%20Object%20Reference) (OtherActor :type Actor%20Object%20Reference) (OtherComp :type Primitive%20Component%20Object%20Reference) (OtherBodyIndex :type Integer))
  (Variables|Default|SetCurrentDrawerIndex 0))

(event OnComponentEndOverlap(Trigger_Drawer2)
  (params (OverlappedComponent :type Primitive%20Component%20Object%20Reference) (OtherActor :type Actor%20Object%20Reference) (OtherComp :type Primitive%20Component%20Object%20Reference) (OtherBodyIndex :type Integer))
  (Variables|Default|SetCurrentDrawerIndex 0))

(event EventBeginPlay
  (Variables|Default|SetDrawer1_StartPos (Variables|/Script/Engine.SceneComponent|GetRelativeLocation (Variables|Default|GetDrawer_1)))
  (Variables|Default|SetDrawer2_StartPos (Variables|/Script/Engine.SceneComponent|GetRelativeLocation (Variables|Default|GetDrawer_2))))

(event Collision|EventActorBeginOverlap
  (params (OtherActor :type Actor%20Object%20Reference)))

(event EventTick
  (params (DeltaSeconds :type Float%20%28single-precision%29)))

(event Input|KeyboardEvents|F
  (params (Key :type Key%20Structure :default "None"))
  (bind _drawer1_startpos (Variables|Default|GetDrawer1_StartPos))
  (bind _drawer2_startpos (Variables|Default|GetDrawer2_StartPos))
  (:Pressed
    (switch int (Variables|Default|GetCurrentDrawerIndex)
      (:1
        (Utilities|FlowControl|Sequence
          (:then_0
            (Variables|Default|SetIsDrawer1_Open true)
            (bind _foundwidgets (Widget|GetAllWidgetsOfClass "/Game/UI/Blueprints/WBP_InteractionPrompt.WBP_InteractionPrompt_C" true))
            (for _array_element _foundwidgets
              (Widget|RemovefromParent _array_element)))
          (:then_1
            (bind _float_track (Timeline|Timeline_Drawer1 Play)
              (:Update
                (Transformation|SetRelativeLocation (Variables|Default|GetDrawer_1) (Math|Vector|Lerp(Vector) _drawer1_startpos (+ _drawer1_startpos (Variables|Default|GetDrawerOffset)) _float_track) false false))))))
      (:2
        (Utilities|FlowControl|Sequence
          (:then_0
            (Variables|Default|SetIsDrawer2_open true)
            (bind _foundwidgets_2 (Widget|GetAllWidgetsOfClass "/Game/UI/Blueprints/WBP_InteractionPrompt.WBP_InteractionPrompt_C" true))
            (for _array_element_2 _foundwidgets_2
              (Widget|RemovefromParent _array_element_2)))
          (:then_1
            (bind _float_track_2 (Timeline|Timeline_drawer%202 Play)
              (:Update
                (Transformation|SetRelativeLocation (Variables|Default|GetDrawer_2) (Math|Vector|Lerp(Vector) _drawer2_startpos (+ _drawer2_startpos (Variables|Default|GetDrawerOffset)) _float_track_2) false false)))))))))

(event Input|KeyboardEvents|C
  (params (Key :type Key%20Structure :default "None"))
  (:Pressed
    (bind _asbp_placement_spot (Utilities|Casting|CastToBP_PlacementSpot (Variables|/Script/Engine.ChildActorComponent|GetChildActor (Variables|Default|GetBP_PlacementSpot_Handle))))
    (bind _asbp_placement_spot_2 (Utilities|Casting|CastToBP_PlacementSpot (Variables|/Script/Engine.ChildActorComponent|GetChildActor (Variables|Default|GetBP_PlacementSpot_HammerHead))))
    (if (and (Variables|/Game/Blueprints/BP_PlacementSpot.BP_PlacementSpot_C|GetIsItemPlaced _asbp_placement_spot) (Variables|/Game/Blueprints/BP_PlacementSpot.BP_PlacementSpot_C|GetIsItemPlaced _asbp_placement_spot_2))
      (Components|DestroyComponent (Variables|Default|GetBP_PlacementSpot_Handle))
      (Components|DestroyComponent (Variables|Default|GetBP_PlacementSpot_HammerHead))
      (Game|SpawnActorfromClass "/Game/Blueprints/BP_WholeHammer.BP_WholeHammer_C" (Transformation|GetWorldTransform (Variables|Default|GetCraftingZone)) "AlwaysSpawn" "MultiplyWithRoot" 0 0)
      (else
        (bind _returnvalue (UserInterface|CreateWidget "/Game/UI/Blueprints/WBP_FlashMessage.WBP_FlashMessage_C" 0 "Missing parts!"))
        (UserInterface|Viewport|AddtoViewport _returnvalue 0)))))

(fn ConstructionScript)