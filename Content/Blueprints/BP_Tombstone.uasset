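; BP_Tombstone is the tombstone interactable that ends Level 2 when the player places the tombstone scroll on it.
; Its trigger shows an interaction prompt once the character's bird puzzle is solved, and clears it on exit.
; PlaceScroll runs once if the player holds the scroll, revealing an image and removing the item from inventory and HUD.
; It then clears prompts and shows the Level 2 end widget after a short delay.
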(event OnComponentBeginOverlap(Trigger)
  (params (OverlappedComponent :type Primitive%20Component%20Object%20Reference) (OtherActor :type Actor%20Object%20Reference) (OtherComp :type Primitive%20Component%20Object%20Reference) (OtherBodyIndex :type Integer) (bFromSweep :type Boolean) (SweepResult :type Hit%20Result%20Structure%20%28by%20ref%29))
  (bind _asbp_third_person_character (Utilities|Casting|CastToBP_ThirdPersonCharacter OtherActor))
  (if (Variables|/Game/ThirdPerson/Blueprints/BP_ThirdPersonCharacter.BP_ThirdPersonCharacter_C|GetIsBirdSolved _asbp_third_person_character)
    (bind _returnvalue (UserInterface|CreateWidget "/Game/UI/Blueprints/WBP_InteractionPrompt_E.WBP_InteractionPrompt_E_C"))
    (bind _output_get (Variables|Default|SetInteractionWidgetRef _returnvalue))
    (UserInterface|Viewport|AddtoViewport _output_get 0)))

(event OnComponentEndOverlap(Trigger)
  (params (OverlappedComponent :type Primitive%20Component%20Object%20Reference) (OtherActor :type Actor%20Object%20Reference) (OtherComp :type Primitive%20Component%20Object%20Reference) (OtherBodyIndex :type Integer))
  (Utilities|Casting|CastToBP_ThirdPersonCharacter OtherActor)
  (bind _foundwidgets (Widget|GetAllWidgetsOfClass "/Game/UI/Blueprints/WBP_InteractionPrompt_E.WBP_InteractionPrompt_E_C" true))
  (for _array_element _foundwidgets
    (Widget|RemovefromParent _array_element)))

(event Custom|PlaceScroll
  (if (not (Variables|Default|GetIsScrollPlaced))
    (bind _asbp_third_person_character (Utilities|Casting|CastToBP_ThirdPersonCharacter (Game|GetPlayerCharacter 0)))
    (if (Variables|/Game/ThirdPerson/Blueprints/BP_ThirdPersonCharacter.BP_ThirdPersonCharacter_C|GetHasTombstoneScroll _asbp_third_person_character)
      (Variables|Default|SetIsScrollPlaced true)
      (Development|SetHiddeninGame (Variables|Default|GetImg) false false)
      (bind _asbp_third_person_character_2 (Utilities|Casting|CastToBP_ThirdPersonCharacter (Game|GetPlayerCharacter 0)))
      (bind _aswbp_inventory_hud (Utilities|Casting|CastToWBP_InventoryHUD (Variables|/Game/ThirdPerson/Blueprints/BP_ThirdPersonCharacter.BP_ThirdPersonCharacter_C|GetInventoryHUD_Ref _asbp_third_person_character_2)))
      (Default|ClearSlotIcon _aswbp_inventory_hud 1)
      (Default|RemoveItem (Variables|/Game/ThirdPerson/Blueprints/BP_ThirdPersonCharacter.BP_ThirdPersonCharacter_C|GetBPC_Inventory _asbp_third_person_character_2) 1)
      (bind _foundwidgets (Widget|GetAllWidgetsOfClass "/Game/UI/Blueprints/WBP_InteractionPrompt_E.WBP_InteractionPrompt_E_C" true))
      (for _array_element _foundwidgets
        (Widget|RemovefromParent _array_element)
        (Utilities|FlowControl|Delay 2.0)
        (bind _returnvalue (UserInterface|CreateWidget "/Game/UI/Blueprints/WBP_Level2_End.WBP_Level2_End_C"))
        (UserInterface|Viewport|AddtoViewport _returnvalue 0))
      (Utilities|FlowControl|Delay 2.0)
      (bind _returnvalue_2 (UserInterface|CreateWidget "/Game/UI/Blueprints/WBP_Level2_End.WBP_Level2_End_C"))
      (UserInterface|Viewport|AddtoViewport _returnvalue_2 0))))

(event EventBeginPlay)

(event Collision|EventActorBeginOverlap
  (params (OtherActor :type Actor%20Object%20Reference)))

(event EventTick
  (params (DeltaSeconds :type Float%20%28single-precision%29)))

(fn ConstructionScript)