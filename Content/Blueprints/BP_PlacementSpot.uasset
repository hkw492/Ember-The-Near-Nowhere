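; Placement spot actor where the player presses E inside a trigger zone to place a required inventory item.
; Trigger overlap toggles input, and E checks the character's inventory, showing a "Missing Items!" flash message if absent.
; On success the hologram mesh takes a hard-coded hammer/anvil material and collision, the item leaves inventory and HUD, and OnItemPlaced is called.
; An older spawn-and-destroy placement path remains unconnected.
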(event OnComponentBeginOverlap(TriggerZone)
  (params (OverlappedComponent :type Primitive%20Component%20Object%20Reference) (OtherActor :type Actor%20Object%20Reference) (OtherComp :type Primitive%20Component%20Object%20Reference) (OtherBodyIndex :type Integer) (bFromSweep :type Boolean) (SweepResult :type Hit%20Result%20Structure%20%28by%20ref%29))
  (Input|EnableInput (Game|GetPlayerController 0)))

(event OnComponentEndOverlap(TriggerZone)
  (params (OverlappedComponent :type Primitive%20Component%20Object%20Reference) (OtherActor :type Actor%20Object%20Reference) (OtherComp :type Primitive%20Component%20Object%20Reference) (OtherBodyIndex :type Integer))
  (Input|DisableInput (Game|GetPlayerController 0)))

(event EventBeginPlay)

(event Collision|EventActorBeginOverlap
  (params (OtherActor :type Actor%20Object%20Reference)))

(event EventTick
  (params (DeltaSeconds :type Float%20%28single-precision%29)))

(event Input|KeyboardEvents|E
  (params (Key :type Key%20Structure :default "None"))
  (bind _hologrammesh (Variables|Default|GetHologramMesh))
  (:Pressed
    (bind _asbp_third_person_character (Utilities|Casting|CastToBP_ThirdPersonCharacter (Game|GetPlayerCharacter 0)))
    (bind _hasit (Default|HasItem (Variables|/Game/ThirdPerson/Blueprints/BP_ThirdPersonCharacter.BP_ThirdPersonCharacter_C|GetBPC_Inventory _asbp_third_person_character) (Variables|Default|GetRequiredItemID)))
    (if _hasit
      (Rendering|Material|SetMaterial _hologrammesh 0 "/Game/HandPaintedEnvironment/Assets/Materials/Summer_mat/Hammer_anvil.Hammer_anvil")
      (Collision|SetCollisionEnabled _hologrammesh "QueryAndPhysics")
      (bind _asbp_third_person_character_2 (Utilities|Casting|CastToBP_ThirdPersonCharacter (Game|GetPlayerCharacter 0)))
      (bind _slotindex (Default|FindSlotOfItem (Variables|/Game/ThirdPerson/Blueprints/BP_ThirdPersonCharacter.BP_ThirdPersonCharacter_C|GetBPC_Inventory _asbp_third_person_character_2) (Variables|Default|GetRequiredItemID)))
      (bind _aswbp_inventory_hud (Utilities|Casting|CastToWBP_InventoryHUD (Variables|/Game/ThirdPerson/Blueprints/BP_ThirdPersonCharacter.BP_ThirdPersonCharacter_C|GetInventoryHUD_Ref _asbp_third_person_character_2)))
      (Default|ClearSlotIcon _aswbp_inventory_hud _slotindex)
      (Default|RemoveItem (Variables|/Game/ThirdPerson/Blueprints/BP_ThirdPersonCharacter.BP_ThirdPersonCharacter_C|GetBPC_Inventory _asbp_third_person_character_2) _slotindex)
      (Variables|Default|SetIsItemPlaced true)
      (Default|CallOnItemPlaced)
      (Input|DisableInput (Game|GetPlayerController 0))
      (else
        (bind _returnvalue (UserInterface|CreateWidget "/Game/UI/Blueprints/WBP_FlashMessage.WBP_FlashMessage_C" 0 "Missing Items!"))
        (UserInterface|Viewport|AddtoViewport _returnvalue 0)))))

(fn ConstructionScript)