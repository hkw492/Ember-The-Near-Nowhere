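; Sliding door puzzle that needs a handle, then a key, both consumed from the player's inventory and HUD.
; An overlap sphere shows an interaction prompt and enables F input while the door is closed.
; F attaches the handle, then a later press with the key slides the door by DoorOffset via a timeline lerp.
; Objective text reports missing items, and switches to finding objects on every timeline update.
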(event OnComponentBeginOverlap(Sphere)
  (params (OverlappedComponent :type Primitive%20Component%20Object%20Reference) (OtherActor :type Actor%20Object%20Reference) (OtherComp :type Primitive%20Component%20Object%20Reference) (OtherBodyIndex :type Integer) (bFromSweep :type Boolean) (SweepResult :type Hit%20Result%20Structure%20%28by%20ref%29))
  (bind _returnvalue (Game|GetPlayerController 0))
  (Utilities|Casting|CastToBP_ThirdPersonCharacter OtherActor)
  (if (not (Variables|Default|GetIsDoorOpen))
    (bind _returnvalue_2 (UserInterface|CreateWidget "/Game/UI/Blueprints/WBP_InteractionPrompt.WBP_InteractionPrompt_C" _returnvalue))
    (bind _output_get (Variables|Default|SetInteractWidgetInstance _returnvalue_2))
    (UserInterface|Viewport|AddtoViewport _output_get 0)
    (Input|EnableInput _returnvalue)))

(event OnComponentEndOverlap(Sphere)
  (params (OverlappedComponent :type Primitive%20Component%20Object%20Reference) (OtherActor :type Actor%20Object%20Reference) (OtherComp :type Primitive%20Component%20Object%20Reference) (OtherBodyIndex :type Integer))
  (Utilities|Casting|CastToBP_ThirdPersonCharacter OtherActor)
  (bind _foundwidgets (Widget|GetAllWidgetsOfClass "/Game/UI/Blueprints/WBP_InteractionPrompt.WBP_InteractionPrompt_C" true))
  (for _array_element _foundwidgets
    (Widget|RemovefromParent _array_element))
  (Input|DisableInput (Game|GetPlayerController 0)))

(event EventBeginPlay
  (Variables|Default|SetInitialLocation (Transformation|GetActorLocation)))

(event Collision|EventActorBeginOverlap
  (params (OtherActor :type Actor%20Object%20Reference)))

(event EventTick
  (params (DeltaSeconds :type Float%20%28single-precision%29)))

(event Input|KeyboardEvents|F
  (params (Key :type Key%20Structure :default "None"))
  (bind _initiallocation (Variables|Default|GetInitialLocation))
  (:Pressed
    (if (Variables|Default|GetIsHandleAttached)
      (bind _asbp_third_person_character (Utilities|Casting|CastToBP_ThirdPersonCharacter (Game|GetPlayerCharacter 0)))
      (bind _slotindex (Default|FindSlotOfItem (Variables|/Game/ThirdPerson/Blueprints/BP_ThirdPersonCharacter.BP_ThirdPersonCharacter_C|GetBPC_Inventory _asbp_third_person_character) (Variables|Default|GetRequiredKeyID)))
      (if (> _slotindex 0)
        (bind _asbp_third_person_character_2 (Utilities|Casting|CastToBP_ThirdPersonCharacter (Game|GetPlayerCharacter 0)))
        (bind _aswbp_inventory_hud (Utilities|Casting|CastToWBP_InventoryHUD (Variables|/Game/ThirdPerson/Blueprints/BP_ThirdPersonCharacter.BP_ThirdPersonCharacter_C|GetInventoryHUD_Ref _asbp_third_person_character_2)))
        (Default|ClearSlotIcon _aswbp_inventory_hud _slotindex)
        (Default|RemoveItem (Variables|/Game/ThirdPerson/Blueprints/BP_ThirdPersonCharacter.BP_ThirdPersonCharacter_C|GetBPC_Inventory _asbp_third_person_character_2) _slotindex)
        (Utilities|FlowControl|Sequence
          (:then_0
            (Variables|Default|SetIsDoorOpen true)
            (bind _foundwidgets (Widget|GetAllWidgetsOfClass "/Game/UI/Blueprints/WBP_InteractionPrompt.WBP_InteractionPrompt_C" true))
            (for _array_element _foundwidgets
              (Widget|RemovefromParent _array_element))
            (Input|DisableInput (Game|GetPlayerController 0)))
          (:then_1
            (bind _float_output (Timeline|DoorMove Play)
              (:Update
                (Transformation|SetActorLocation (Math|Vector|Lerp(Vector) _initiallocation (+ _initiallocation (Variables|Default|GetDoorOffset)) _float_output) false false)
                (bind _asbp_third_person_character_3 (Utilities|Casting|CastToBP_ThirdPersonCharacter (Game|GetPlayerCharacter 0)))
                (Default|UpdateObjective _asbp_third_person_character_3 "Find the Objects")))))
        (else
          (bind _asbp_third_person_character_4 (Utilities|Casting|CastToBP_ThirdPersonCharacter (Game|GetPlayerCharacter 0)))
          (Default|UpdateObjective _asbp_third_person_character_4 "Locked. Find the key")))
      (else
        (bind _asbp_third_person_character_5 (Utilities|Casting|CastToBP_ThirdPersonCharacter (Game|GetPlayerCharacter 0)))
        (bind _slotindex_2 (Default|FindSlotOfItem (Variables|/Game/ThirdPerson/Blueprints/BP_ThirdPersonCharacter.BP_ThirdPersonCharacter_C|GetBPC_Inventory _asbp_third_person_character_5) (Variables|Default|GetRequiredHandleID)))
        (if (> _slotindex_2 0)
          (Variables|Default|SetIsHandleAttached true)
          (Rendering|SetVisibility (Variables|Default|GetDoor_Handle) true false)
          (bind _asbp_third_person_character_6 (Utilities|Casting|CastToBP_ThirdPersonCharacter (Game|GetPlayerCharacter 0)))
          (bind _aswbp_inventory_hud_2 (Utilities|Casting|CastToWBP_InventoryHUD (Variables|/Game/ThirdPerson/Blueprints/BP_ThirdPersonCharacter.BP_ThirdPersonCharacter_C|GetInventoryHUD_Ref _asbp_third_person_character_6)))
          (Default|ClearSlotIcon _aswbp_inventory_hud_2 _slotindex_2)
          (Default|RemoveItem (Variables|/Game/ThirdPerson/Blueprints/BP_ThirdPersonCharacter.BP_ThirdPersonCharacter_C|GetBPC_Inventory _asbp_third_person_character_6) _slotindex_2)
          (else
            (bind _asbp_third_person_character_7 (Utilities|Casting|CastToBP_ThirdPersonCharacter (Game|GetPlayerCharacter 0)))
            (Default|UpdateObjective _asbp_third_person_character_7 "It's broken. Find the handle.")))))))

(fn ConstructionScript)