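; BP_SlidingPlank is an interactable plank that slides open once, with no path to close it.
; MovePlank runs a timeline that lerps the mesh's relative location from its starting point by PlankOffset.
; Highlight events toggle a green overlay material, and CanInteract always returns true.
; The trigger shows an E prompt and enables input for the third-person character, then removes the prompt on exit without disabling input.
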(event OnComponentBeginOverlap(Trigger)
  (params (OverlappedComponent :type Primitive%20Component%20Object%20Reference) (OtherActor :type Actor%20Object%20Reference) (OtherComp :type Primitive%20Component%20Object%20Reference) (OtherBodyIndex :type Integer) (bFromSweep :type Boolean) (SweepResult :type Hit%20Result%20Structure%20%28by%20ref%29))
  (Utilities|Casting|CastToBP_ThirdPersonCharacter OtherActor)
  (bind _returnvalue (UserInterface|CreateWidget "/Game/UI/Blueprints/WBP_InteractionPrompt_E.WBP_InteractionPrompt_E_C"))
  (bind _output_get (Variables|Default|SetInteractRef _returnvalue))
  (UserInterface|Viewport|AddtoViewport _output_get 0)
  (Input|EnableInput (Game|GetPlayerController 0)))

(event OnComponentEndOverlap(Trigger)
  (params (OverlappedComponent :type Primitive%20Component%20Object%20Reference) (OtherActor :type Actor%20Object%20Reference) (OtherComp :type Primitive%20Component%20Object%20Reference) (OtherBodyIndex :type Integer))
  (Utilities|Casting|CastToBP_ThirdPersonCharacter OtherActor)
  (bind _foundwidgets (Widget|GetAllWidgetsOfClass "/Game/UI/Blueprints/WBP_InteractionPrompt_E.WBP_InteractionPrompt_E_C" true))
  (for _array_element _foundwidgets
    (Widget|RemovefromParent _array_element)))

(event Custom|MovePlank
  (bind _initiallocation (Variables|Default|GetInitialLocation))
  (if (not (Variables|Default|GetIsOpen))
    (Variables|Default|SetIsOpen true)
    (bind _plank (Timeline|move%20plank Play)
      (:Update
        (Transformation|SetRelativeLocation (Variables|Default|GetStaticMesh) (Math|Vector|Lerp(Vector) _initiallocation (+ _initiallocation (Variables|Default|GetPlank%20Offset)) _plank) false false)))))

(event EventBeginPlay
  (Variables|Default|SetInitialLocation (Variables|/Script/Engine.SceneComponent|GetRelativeLocation (Variables|Default|GetStaticMesh))))

(event Collision|EventActorBeginOverlap
  (params (OtherActor :type Actor%20Object%20Reference)))

(event EventTick
  (params (DeltaSeconds :type Float%20%28single-precision%29)))

(event EventOnInteractHighlight
  (Rendering|Material|SetOverlayMaterial (Variables|Default|GetStaticMesh) "/Game/Textures/Glow_Box/MI_GreenHighlight.MI_GreenHighlight" :!class /Script/Engine.MeshComponent))

(event EventOnInteractEnd
  (Rendering|Material|SetOverlayMaterial (Variables|Default|GetStaticMesh) 0 :!class /Script/Engine.MeshComponent))

(fn ConstructionScript)

(fn CanInteract
  (return true))