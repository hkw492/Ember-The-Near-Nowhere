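; Swinging sign actor for the stylized village that rocks its static mesh back and forth using a timeline.
; After a configurable delay, the timeline plays and sets itself to loop on each update.
; Its Swinging track, scaled by SwingAmount, drives roll, while InitialTurn plus InitialTurnValue sets yaw.
; Tick feeds the same delay-and-play chain as BeginPlay, so Play is re-issued repeatedly.
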(event EventTick
  (params (DeltaSeconds :type Float%20%28single-precision%29))
  (Utilities|FlowControl|Delay (Variables|Default|GetDelay%20Amount))
  (bind (_direction _swinging _initialturn) (Timeline|Timeline_0 Play)
    (:Update
      (Components|Timeline|SetLooping (Variables|Default|GetTimeline_0) true)
      (Transformation|SetRelativeRotation (Variables|Debug|GetStaticMeshComponent) (Math|Rotator|MakeRotator (* _swinging (Variables|Default|GetSwing%20Amount)) 0.0 (+ _initialturn (Variables|Default|GetInitial%20Turn%20Value))) false false))))

(event EventBeginPlay
  (Utilities|FlowControl|Delay (Variables|Default|GetDelay%20Amount))
  (bind (_direction _swinging _initialturn) (Timeline|Timeline_0 Play)
    (:Update
      (Components|Timeline|SetLooping (Variables|Default|GetTimeline_0) true)
      (Transformation|SetRelativeRotation (Variables|Debug|GetStaticMeshComponent) (Math|Rotator|MakeRotator (* _swinging (Variables|Default|GetSwing%20Amount)) 0.0 (+ _initialturn (Variables|Default|GetInitial%20Turn%20Value))) false false))))

(fn ConstructionScript)